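; Dialogue component for the vending machine that holds Lily's favorite snack.
; It checks BP_Vending's Ready flag and either offers a button push or says the player should get coffee first.
; Pushing the button shows the Munch Bar pickup with a one-time sound cue, and leaving closes the conversation and tells BP_Wall to run WallsDownMessage.
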(fn `Conversation`
  (`self.SetDialogueTreeIndex` "None")
  (`parent.Conversation`))

(fn `Dialogue`
  ;[0.15 0.08514 0.1455 0.5] Create Dialogue and Options that will be added to widget
  (`parent.Dialogue`)
  (switch `name` (`self.ActiveDialogueBranch`)
    (:`Default`
      (bind _returnvalue (`GameplayStatics.GetActorOfClass` "/Game/Kyra/BP/BP_Vending.BP_Vending_C"))
      (if (`/Game/Kyra/BP/BP_Vending.ready` _returnvalue)
        (bind (_state _optionindex) (`self.AddDialogue` "Vending Machine" "*It has Lily's favorite snack*" (`|MakeArray` "*Push button*" :!type "Text")))
        (switch `/Game/Evelyn/Dialogue_Bluprints/Enum_Dialogue` _state
          (:`NewEnumerator0`
            (switch `int` _optionindex
              (:`0`
                (bind _state_2 (`self.AddDialogue` "Vending Machine" "*Munch Bar aqquired*" (`|MakeArray` "*Leave*" :!type "Text")))
                (`|ExecutionSequence`
                  (:`then_0`
                    (switch `/Game/Evelyn/Dialogue_Bluprints/Enum_Dialogue` _state_2
                      (:`NewEnumerator0`
                        (`self.ClearDialogueProgress`) ; Clears
                        (`self.CloseConversation`) ; Ends the conversation, can be restarted....
                        (bind _returnvalue_2 (`GameplayStatics.GetActorOfClass` "/Game/Kyra/BP/BP_Wall.BP_Wall_C"))
                        (message `/Game/Kyra/BP_WallInt.WallsDown` _returnvalue_2))))
                  (:`then_1`
                    (if (`self.PlaySound`)
                      (`GameplayStatics.SpawnSound2D` "/Game/Kyra/Audio/Vending_Cue.Vending_Cue" 1.0 1.0 0.0 null)
                      (set `self.PlaySound` false))))))))
        (else
          (bind _state_3 (`self.AddDialogue` "Vending Machine" "*It has Lily's favorite snack.*" (`|MakeArray` "I should get coffee first." :!type "Text")))
          (switch `/Game/Evelyn/Dialogue_Bluprints/Enum_Dialogue` _state_3
            (:`NewEnumerator0`
              (`self.ClearDialogueProgress`)
              (`self.CloseConversation`))))))))

(fn `NewFunction`)