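; BP_Vending is an interactable vending Blueprint that prompts a thought about getting something for Lilly and runs a dialogue.
; PromptPlayer briefly shows a W_Thoughts widget created at BeginPlay, then sets a Ready flag, which Interact does not check.
; Interact stores the instigator and starts the ACVendingDialogue conversation.
; ConversationClosed notifies that stored instigator through ConversationClosedMessage.
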(event `self.ReceiveBeginPlay`
  (bind _returnvalue (`|CreateWidget` "/Game/UI/W_Thoughts.W_Thoughts_C")))

(event `PromptPlayer`
  (`/Game/UI/W_Thoughts.Think` (stale `self.ReceiveBeginPlay` _returnvalue) "I want to get something for Lilly when she wakes up.")
  (`UserWidget.AddToViewport` (stale `self.ReceiveBeginPlay` _returnvalue) 0)
  (`KismetSystemLibrary.Delay` 3.0)
  (`Widget.RemoveFromParent` (stale `self.ReceiveBeginPlay` _returnvalue))
  (set `self.ready` true))

(event `/Game/Evelyn/Dialogue_Bluprints/BP_Interaction.Interact`
  (params (Instigator :type "Actor Object Reference"))
  (set `self.InteractInstigator` Instigator)
  (`/Game/Evelyn/Dialogue_Bluprints/Dialogues/AC_Dialogue_Base.Conversation` (`self.AC_Vending_Dialogue`)))

(event `/Game/Evelyn/Dialogue_Bluprints/BP_Interaction.Conversation Closed`
  (message `/Game/Evelyn/Dialogue_Bluprints/BP_Interaction.Conversation Closed` (`self.InteractInstigator`)))

(fn `UserConstructionScript`)