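; BP_Wall is a toggleable wall that shows the thought "I don't want to leave yet." on overlap.
; BeginPlay disables the Cube's collision and prepares the thought widget.
; WallsUp enables query and physics collision, then after a short delay lets Cube overlaps add and remove the widget from the viewport.
; WallsDown disables collision again but leaves the TalkYet flag unchanged.
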(event `self.ReceiveBeginPlay`
  (`PrimitiveComponent.SetCollisionEnabled` (`self.Cube`) "NoCollision")
  (bind _returnvalue (`|CreateWidget` "/Game/UI/W_Thoughts.W_Thoughts_C"))
  (`/Game/UI/W_Thoughts.Think` _returnvalue "I don't want to leave yet.")
  (set `self.talkYet` false))

(event `/Game/Kyra/BP_WallInt.wallsUp`
  (`PrimitiveComponent.SetCollisionEnabled` (`self.Cube`) "QueryAndPhysics")
  (`KismetSystemLibrary.Delay` 3.0)
  (set `self.talkYet` true))

(event `self.Cube.OnComponentBeginOverlap`
  (params (OverlappedComponent :type "PrimitiveComponent Object Reference") (OtherActor :type "Actor Object Reference") (OtherComp :type "PrimitiveComponent Object Reference") (OtherBodyIndex :type Integer) (bFromSweep :type Boolean) (SweepResult :type "HitResult Structure (by ref)"))
  (if (`self.talkYet`)
    (`UserWidget.AddToViewport` (stale `self.ReceiveBeginPlay` _returnvalue) 0)))

(event `self.Cube.OnComponentEndOverlap`
  (params (OverlappedComponent :type "PrimitiveComponent Object Reference") (OtherActor :type "Actor Object Reference") (OtherComp :type "PrimitiveComponent Object Reference") (OtherBodyIndex :type Integer))
  (if (`self.talkYet`)
    (`Widget.RemoveFromParent` (stale `self.ReceiveBeginPlay` _returnvalue))))

(event `/Game/Kyra/BP_WallInt.WallsDown`
  (`PrimitiveComponent.SetCollisionEnabled` (`self.Cube`) "NoCollision"))

(fn `UserConstructionScript`)