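; Dialogue component for the character Linda, defining her branching conversation in which she blames the player for Lily being in the hospital.
; It overrides Dialogue, calls the parent, then chains AddDialogue calls that supply lines and player options for the widget, branching on the chosen OptionIndex.
; Both replies lead to a hostile response with a Leave option, which clears dialogue progress and closes the conversation so it can be restarted.
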(fn `Dialogue`
  ;[0.15 0.08514 0.1455 0.5] Create Dialogue and Options that will be added to widget
  (`parent.Dialogue`)
  (switch `int` (`self.DialogueTreeIndex`)
    (:`Default`
      (bind (_state _optionindex) (`self.AddDialogue` "Linda" "It's your fault Lily is in the hospital" (`|MakeArray` "*stays silent*" "Will she be alright?" :!type "Text")))
      (switch `/Game/BluePrints/Dialogue_Bluprints/Enum_Dialogue` _state
        (:`NewEnumerator0`
          (switch `int` _optionindex
            (:`0`
              (bind _state_2 (`self.AddDialogue` "Linda" "Have you nothing to say?! Leave my sight before I do something I regret" (`|MakeArray` "Leave" :!type "Text")))
              (switch `/Game/BluePrints/Dialogue_Bluprints/Enum_Dialogue` _state_2
                (:`NewEnumerator0`
                  (`self.ClearDialogueProgress`) ; Clears
                  (`self.CloseConversation`) ; Ends the conversation, can be restarted....
                )))
            (:`1`
              (bind _state_3 (`self.AddDialogue` "Linda" "As if you deserve to know" (`|MakeArray` "Leave" :!type "Text")))
              (switch `/Game/BluePrints/Dialogue_Bluprints/Enum_Dialogue` _state_3
                (:`NewEnumerator0`
                  (`self.ClearDialogueProgress`)
                  (`self.CloseConversation`))))))))))