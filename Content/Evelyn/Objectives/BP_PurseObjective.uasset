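; Objective actor, named for a purse objective, that shows on-screen objective and completion notices through a W_Objective widget created at BeginPlay.
; ObjectiveAppears runs once, filling the widget from its text variables, fading it in and out around a delay, and setting ObjectiveProgress.
; CompletedObjective replays the fade with completion text and restyled content.
; The construction script sizes ObjectiveBox, but overlap is unused here, so neither custom event is called within this graph.
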(event `self.ReceiveBeginPlay`
  (bind _returnvalue (`|CreateWidget` "/Game/UI/W_Objective.W_Objective_C" null "Objective" "Go to Cafeteria"))
  (set `self.ObjectiveWidgetRef` _returnvalue))

(event `ObjectiveAppears`
  (bind _objectivewidgetref (`self.ObjectiveWidgetRef`))
  (bind _objectivewidgetref_2 (`self.ObjectiveWidgetRef`))
  (bind _objectivefade (`/Game/UI/W_Objective.ObjectiveFade` _objectivewidgetref))
  (`/Engine/EditorBlueprintResources/StandardMacros.DoOnce` false
    (:`Completed`
      (set `/Game/UI/W_Objective.ObjectiveTitleText` (`self.ObjectiveTitleText`) _objectivewidgetref_2)
      (set `/Game/UI/W_Objective.ObjectiveContentText` (`self.ObjectiveContentText`) _objectivewidgetref_2)
      (`TextBlock.SetColorAndOpacity` (`/Game/UI/W_Objective.ObjectiveContent` _objectivewidgetref_2) (make `SlateColor` (make `LinearColor` 1.0 1.0)))
      (`UserWidget.AddToViewport` _objectivewidgetref 0)
      (`UserWidget.PlayAnimation` _objectivewidgetref _objectivefade 0.0 1 "Forward" 1.0 false)
      (`KismetSystemLibrary.Delay` 5.0)
      (`UserWidget.PlayAnimation` _objectivewidgetref _objectivefade 0.0 1 "Reverse" 1.0 false)
      (set `self.ObjectiveProgress` true))))

(event `CompletedObjective`
  (bind _objectivewidgetref (`self.ObjectiveWidgetRef`))
  (bind _objectivewidgetref_2 (`self.ObjectiveWidgetRef`))
  (bind _objectivefade (`/Game/UI/W_Objective.ObjectiveFade` _objectivewidgetref))
  (set `/Game/UI/W_Objective.ObjectiveTitleText` "Completed Objective" _objectivewidgetref_2)
  (`TextBlock.SetColorAndOpacity` (`/Game/UI/W_Objective.ObjectiveContent` _objectivewidgetref_2) (make `SlateColor` (make `LinearColor` 1.0 0.0 1.0 0.5)))
  (`UserWidget.PlayAnimation` _objectivewidgetref _objectivefade 0.0 1 "Forward" 1.0 false)
  (`KismetSystemLibrary.Delay` 3.0)
  (`UserWidget.PlayAnimation` _objectivewidgetref _objectivefade 0.0 1 "Reverse" 1.0 false))

(fn `UserConstructionScript`
  (locals (NewLocalVar :type "BoxComponent Object Reference"))
  (`BoxComponent.SetBoxExtent` (`self.ObjectiveBox`) (`self.ObjeciveBoxSize`) true))