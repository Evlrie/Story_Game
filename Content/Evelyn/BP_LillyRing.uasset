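; BP_LillyRing is the pickup for Lilly's lost ring, which advances the story when the player interacts with it.
; Interact shows a thought widget and has BP_DoctorSpawnManager spawn the doctor.
; After a short delay it calls the character's ConversationClosedMessage, triggers a BP_Intercom announcement and destroys itself.
; The actor is destroyed before PromptPlayer's longer delay ends, so that event's widget removal and Ready flag are never reached.
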(event `self.ReceiveBeginPlay`)

(event `Prompt player`
  (bind _returnvalue (`|CreateWidget` "/Game/UI/W_Thoughts.W_Thoughts_C"))
  (`/Game/UI/W_Thoughts.Think` _returnvalue "Thank goodness I found Lilly's ring....she would have been so upset.")
  (`UserWidget.AddToViewport` _returnvalue 0)
  (`KismetSystemLibrary.Delay` 2.0)
  (`Widget.RemoveFromParent` _returnvalue)
  (set `self.ready` true))

(event `/Game/Evelyn/Dialogue_Bluprints/BP_Interaction.Interact`
  (params (Instigator :type "Actor Object Reference"))
  (set `self.picked up` true)
  (`KismetSystemLibrary.PrintString` "Hello")
  (`self.Prompt player`)
  ;[0.1465 0.06241 0.15 0.5] After picking up ring will spawn doctor
  (bind _returnvalue (`GameplayStatics.GetActorOfClass` "/Game/Evelyn/Dialogue_Bluprints/BP_DoctorSpawnManager.BP_DoctorSpawnManager_C"))
  (`/Game/Evelyn/Dialogue_Bluprints/BP_DoctorSpawnManager.Spawn Doctor` _returnvalue)
  (`KismetSystemLibrary.Delay` 0.2)
  (bind _returnvalue_2 (`GameplayStatics.GetActorOfClass` "/Game/ThirdPerson/Blueprints/BP_ThirdPersonCharacter.BP_ThirdPersonCharacter_C"))
  (message `/Game/Evelyn/Dialogue_Bluprints/BP_Interaction.Conversation Closed` _returnvalue_2)
  (`KismetSystemLibrary.PrintString` "Hello")
  (bind _returnvalue_3 (`GameplayStatics.GetActorOfClass` "/Game/Kyra/BP/BP_Intercom.BP_Intercom_C"))
  (`/Game/Kyra/BP/BP_Intercom.makeAnnouncement` _returnvalue_3)
  (`self.K2_DestroyActor`))

(fn `UserConstructionScript`)