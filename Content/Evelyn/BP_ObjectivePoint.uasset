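; BP_ObjectivePoint is a trigger point that shows an objective on screen when the player enters its box, sized from a variable at construction.
; It creates a W_Objective widget on BeginPlay, then on first player overlap fills in the text, fades it in and out, and sets ObjectiveProgress.
; CompletedObjective reuses the widget, retitling it as completed with dimmed content text and replaying the timed fade.
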(event `self.ReceiveBeginPlay`
  (bind _returnvalue (`|CreateWidget` "/Game/UI/W_Objective.W_Objective_C" null (`self.ObjectiveTitleText`) (`self.ObjectiveTitleText`)))
  (set `self.ObjectiveWidgetRef` _returnvalue))

(event `self.ObjectiveBox.OnComponentBeginOverlap`
  (params (OverlappedComponent :type "PrimitiveComponent Object Reference") (OtherActor :type "Actor Object Reference") (OtherComp :type "PrimitiveComponent Object Reference") (OtherBodyIndex :type Integer) (bFromSweep :type Boolean) (SweepResult :type "HitResult Structure (by ref)"))
  (bind _objectivewidgetref (`self.ObjectiveWidgetRef`))
  (bind _objectivewidgetref_2 (`self.ObjectiveWidgetRef`))
  (bind _objectivefade (`/Game/UI/W_Objective.ObjectiveFade` _objectivewidgetref_2))
  (if (== OtherActor (`GameplayStatics.GetPlayerCharacter` 0))
    (`/Engine/EditorBlueprintResources/StandardMacros.DoOnce` false
      (:`Completed`
        (set `/Game/UI/W_Objective.ObjectTitleText` (`self.ObjectiveTitleText`) _objectivewidgetref)
        (set `/Game/UI/W_Objective.ObjectiveContentText` (`self.ObjectiveContentText`) _objectivewidgetref)
        (`TextBlock.SetColorAndOpacity` (`/Game/UI/W_Objective.ContentText` _objectivewidgetref) (make `SlateColor` (make `LinearColor` 1.0 1.0 1.0 1.0)))
        (`UserWidget.AddToViewport` _objectivewidgetref_2 0)
        (`UserWidget.PlayAnimation` _objectivewidgetref_2 _objectivefade 0.0 1 "Forward" 1.0 false)
        (`KismetSystemLibrary.Delay` 5.0)
        (`UserWidget.PlayAnimation` _objectivewidgetref_2 _objectivefade 0.0 1 "Reverse" 1.0 false)
        (set `self.ObjectiveProgress` true)))))

(event `Completed Objective`
  (bind _objectivewidgetref (`self.ObjectiveWidgetRef`))
  (bind _objectivefade (`/Game/UI/W_Objective.ObjectiveFade` _objectivewidgetref))
  (set `/Game/UI/W_Objective.ObjectTitleText` "Completed Objective" (`self.ObjectiveWidgetRef`))
  (`TextBlock.SetColorAndOpacity` (`/Game/UI/W_Objective.ContentText` _objectivewidgetref) (make `SlateColor` (make `LinearColor` 1.0 1.0 1.0 0.5)))
  (`UserWidget.PlayAnimation` _objectivewidgetref _objectivefade 0.0 1 "Forward" 1.0 false)
  (`KismetSystemLibrary.Delay` 3.0)
  (`UserWidget.PlayAnimation` _objectivewidgetref _objectivefade 0.0 1 "Reverse" 1.0 false))

(fn `UserConstructionScript`
  (`BoxComponent.SetBoxExtent` (`self.ObjectiveBox`) (`self.Objective Box Size`) true))