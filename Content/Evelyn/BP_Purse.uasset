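; BP_Purse is an interactable purse that starts a dialogue and can reveal the purse objective.
; Interact stores the instigator, starts the conversation on its ACPurseDialogue component, flags itself as interacted and prints a debug message.
; When the conversation closes, it notifies the instigator, then calls ObjectiveAppears on BP_PurseObjective if BP_Coffee was already interacted with.
; Both of those actors are found by class lookup.
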(event `self.Interact`
  (params (Instigator :type "Actor Object Reference"))
  (set `self.InteractInstigator` Instigator)
  (`/Game/Evelyn/Dialogue_Bluprints/Dialogues/AC_Dialogue_Base.Conversation` (`self.AC_Purse_Dialogue`))
  (set `self.Interacted` true)
  (`KismetSystemLibrary.PrintString` "Has interacted"))

(event `self.Conversation Closed`
  (message `/Game/Evelyn/Dialogue_Bluprints/BP_Interaction.Conversation Closed` (`self.InteractInstigator`))
  (bind _returnvalue (`GameplayStatics.GetActorOfClass` "/Game/Kyra/BP/BP_Coffee.BP_Coffee_C"))
  (if (`/Game/Kyra/BP/BP_Coffee.Interacted` _returnvalue)
    (bind _returnvalue_2 (`GameplayStatics.GetActorOfClass` "/Game/Evelyn/Objectives/BP_PurseObjective.BP_PurseObjective_C"))
    (`/Game/Evelyn/Objectives/BP_PurseObjective.ObjectiveAppears` _returnvalue_2)))

(fn `UserConstructionScript`)