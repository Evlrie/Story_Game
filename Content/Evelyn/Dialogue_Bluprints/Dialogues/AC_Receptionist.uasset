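; Dialogue asset for the hospital receptionist nurse, who turns away the player's request to see Lily and suggests waiting or getting coffee.
; Overrides the parent Dialogue function, nesting AddDialogue calls that each supply a line and reply options, advancing on the returned state and option index.
; Both the full exchange and the early Leave option clear progress and close the conversation, which can be restarted.
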(fn `Dialogue`
  ;[0.15 0.08514 0.1455 0.5] Create Dialogue and Options that will be added to widget
  (`parent.Dialogue`)
  (switch `name` (`self.ActiveDialogueBranch`)
    (:`Default`
      (bind (_state _optionindex) (`self.AddDialogue` "Nurse" "Are you alright?" (`|MakeArray` "Can I please see Lily." "Leave" :!type "Text")))
      (switch `/Game/Evelyn/Dialogue_Bluprints/Enum_Dialogue` _state
        (:`NewEnumerator0`
          (switch `int` _optionindex
            (:`0`
              (bind (_state_2 _optionindex_2) (`self.AddDialogue` "Nurse" "I'm sorry, but the doctor said no visitors. " (`|MakeArray` "Please... I need to be there for her." :!type "Text")))
              (switch `/Game/Evelyn/Dialogue_Bluprints/Enum_Dialogue` _state_2
                (:`NewEnumerator0`
                  (switch `int` _optionindex_2
                    (:`0`
                      (bind (_state_3 _optionindex_3) (`self.AddDialogue` "Nurse" "The best you can do for her is wait here. Maybe go get some coffee from the cafeteria." (`|MakeArray` "Ok..." :!type "Text")))
                      (switch `/Game/Evelyn/Dialogue_Bluprints/Enum_Dialogue` _state_3
                        (:`NewEnumerator0`
                          (switch `int` _optionindex_3
                            (:`0`
                              (bind _state_4 (`self.AddDialogue` "Nurse" "You will be the first to know if her condition changes. Let us know if you need anything in the meantime." (`|MakeArray` "Thank you...." :!type "Text")))
                              (switch `/Game/Evelyn/Dialogue_Bluprints/Enum_Dialogue` _state_4
                                (:`NewEnumerator0`
                                  (`self.ClearDialogueProgress`) ; Clears
                                  (`self.CloseConversation`) ; Ends the conversation, can be restarted....
                                )))))))))))
            (:`1`
              (`self.ClearDialogueProgress`) ; Clears
              (`self.CloseConversation`) ; Ends the conversation, can be restarted....
            )))))))