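; Dialogue component for the cafeteria nurse NPC, building a branching conversation through chained AddDialogue calls.
; After the greeting, it reads Interacted on BP_Coffee and NPC_CafeteriaLady: if only the coffee is used, the nurse points the player to the kitchen for machine help.
; Otherwise the nurse asks after the player, opening an escalating confession whose crying options share a repeatable loop.
; Exit options clear progress and close the conversation.
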(fn `Conversation`
  (`self.SetDialogueTreeIndex` "None")
  (`parent.Conversation`))

(fn `Dialogue`
  ;[0.15 0.08514 0.1455 0.5] Create Dialogue and Options that will be added to widget
  (`parent.Dialogue`)
  (switch `name` (`self.ActiveDialogueBranch`)
    (:`Default`
      (bind _state (`self.AddDialogue` "Person" "Good afternoon" (`|MakeArray` "Hey" :!type "Text")))
      (switch `/Game/Evelyn/Dialogue_Bluprints/Enum_Dialogue` _state
        (:`NewEnumerator0`
          (bind _returnvalue (`GameplayStatics.GetActorOfClass` "/Game/Kyra/BP/BP_Coffee.BP_Coffee_C"))
          (if (`/Game/Kyra/BP/BP_Coffee.Interacted` _returnvalue)
            (bind _returnvalue_2 (`GameplayStatics.GetActorOfClass` "/Game/Evelyn/Dialogue_Bluprints/NPCs/NPC_CafeteriaLady.NPC_CafeteriaLady_C"))
            (if (`/Game/Evelyn/Dialogue_Bluprints/NPCs/NPC_CafeteriaLady.Interacted` _returnvalue_2)
              (bind (_state_2 _optionindex) (`self.AddDialogue` "Person" "Is everything okay?" (`|MakeArray` "Sure..." "Not even slightly." "*Leave*" :!type "Text") :!label _label))
              (switch `/Game/Evelyn/Dialogue_Bluprints/Enum_Dialogue` _state_2
                (:`NewEnumerator0`
                  (switch `int` _optionindex
                    (:`0`
                      (bind _state_3 (`self.AddDialogue` "Person" "Good to hear. Have a nice day!" (`|MakeArray` "*Leave*" :!type "Text")))
                      (switch `/Game/Evelyn/Dialogue_Bluprints/Enum_Dialogue` _state_3
                        (:`NewEnumerator0`
                          (`self.ClearDialogueProgress` :!label _label_2) ; Clears
                          (`self.CloseConversation`) ; Ends the conversation, can be restarted....
                        )))
                    (:`1`
                      (bind (_state_4 _optionindex_2) (`self.AddDialogue` "Person" "Oh, well I'm sorry to hear that..." (`|MakeArray` "I got in a wreck..." "*Cry hysterically*" "*Leave*" :!type "Text")))
                      (switch `/Game/Evelyn/Dialogue_Bluprints/Enum_Dialogue` _state_4
                        (:`NewEnumerator0`
                          (switch `int` _optionindex_2
                            (:`0`
                              (bind (_state_5 _optionindex_3) (`self.AddDialogue` "Person" "Woah, uhm..." (`|MakeArray` "And my fiance was in the car..." "*Cry hysterically*" "*Leave*" :!type "Text")))
                              (switch `/Game/Evelyn/Dialogue_Bluprints/Enum_Dialogue` _state_5
                                (:`NewEnumerator0`
                                  (switch `int` _optionindex_3
                                    (:`0`
                                      (bind (_state_6 _optionindex_4) (`self.AddDialogue` "Person" "Oh... Jeez" (`|MakeArray` "And the doctors won't let me go see her..." "*Cry hysterically*" "*Leave*" :!type "Text")))
                                      (switch `/Game/Evelyn/Dialogue_Bluprints/Enum_Dialogue` _state_6
                                        (:`NewEnumerator0`
                                          (switch `int` _optionindex_4
                                            (:`0`
                                              (bind (_state_7 _optionindex_5) (`self.AddDialogue` "Person" "I'm sorry to hear that..." (`|MakeArray` "And her mother hates me now..." "*Cry hysterically*" "*Leave*" :!type "Text")))
                                              (switch `/Game/Evelyn/Dialogue_Bluprints/Enum_Dialogue` _state_7
                                                (:`NewEnumerator0`
                                                  (switch `int` _optionindex_5
                                                    (:`0`
                                                      (bind (_state_8 _optionindex_6) (`self.AddDialogue` "Person" "Gosh!" (`|MakeArray` "I don't know what I'm gonna do..." "*Cry hysterically*" "*Leave*" :!type "Text")))
                                                      (switch `/Game/Evelyn/Dialogue_Bluprints/Enum_Dialogue` _state_8
                                                        (:`NewEnumerator0`
                                                          (switch `int` _optionindex_6
                                                            (:`0`
                                                              (bind (_state_9 _optionindex_7) (`self.AddDialogue` "Person" "Yeah, that's crazy..." (`|MakeArray` "*Cry hysterically*" "*Leave*" :!type "Text")))
                                                              (switch `/Game/Evelyn/Dialogue_Bluprints/Enum_Dialogue` _state_9
                                                                (:`NewEnumerator0`
                                                                  (switch `int` _optionindex_7
                                                                    (:`0`
                                                                      (bind (_state_10 _optionindex_8) (`self.AddDialogue` "Person" "uh, there there!" (`|MakeArray` "*Keep crying*" "-Sniff- *Leave*" :!type "Text") :!label _label_3))
                                                                      (switch `/Game/Evelyn/Dialogue_Bluprints/Enum_Dialogue` _state_10
                                                                        (:`NewEnumerator0`
                                                                          (switch `int` _optionindex_8
                                                                            (:`0`
                                                                              (bind (_state_11 _optionindex_9) (`self.AddDialogue` "Person" "*Awkwardly bites sandwich*" (`|MakeArray` "*Keep crying*" "-Sniff- *Leave*" :!type "Text")))
                                                                              (switch `/Game/Evelyn/Dialogue_Bluprints/Enum_Dialogue` _state_11
                                                                                (:`NewEnumerator0`
                                                                                  (switch `int` _optionindex_9
                                                                                    (:`0`
                                                                                      (goto _label_3))
                                                                                    (:`1`
                                                                                      _)))))
                                                                            (:`1`
                                                                              _)))))
                                                                    (:`1`
                                                                      _)))))
                                                            (:`1`
                                                              (goto _label_3))
                                                            (:`2`
                                                              _)))))
                                                    (:`1`
                                                      (goto _label_3))
                                                    (:`2`
                                                      _)))))
                                            (:`1`
                                              (goto _label_3))
                                            (:`2`
                                              _)))))
                                    (:`1`
                                      (goto _label_3))
                                    (:`2`
                                      _)))))
                            (:`1`
                              (goto _label_3))
                            (:`2`
                              _))
                          (`self.ClearDialogueProgress` :!label _label_4)
                          (`self.CloseConversation`))))
                    (:`2`
                      (goto _label_4)))))
              (else
                (bind (_state_12 _optionindex_10) (`self.AddDialogue` "Person" "Can I help you?" (`|MakeArray` "Do you know how to work the coffee machine?" :!type "Text")))
                (switch `/Game/Evelyn/Dialogue_Bluprints/Enum_Dialogue` _state_12
                  (:`NewEnumerator0`
                    (switch `int` _optionindex_10
                      (:`0`
                        (bind _state_13 (`self.AddDialogue` "Person" "No, but someone in the kitchen might." (`|MakeArray` "Right, thanks." :!type "Text")))
                        (switch `/Game/Evelyn/Dialogue_Bluprints/Enum_Dialogue` _state_13
                          (:`NewEnumerator0`
                            (goto _label_2)))))))))
            (else
              (goto _label))))))))

(fn `NewFunction`)