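; Dialogue component for the Cafeteria Lady NPC, defining her short conversation with the player.
; Overrides Dialogue to chain AddDialogue nodes, each advancing on its Pass Through state.
; After a greeting, BP_Coffee's Interacted flag picks the branch: advice to whack the broken coffee machine, or a suggestion to get a drink.
; Both branches clear progress and close the conversation, which can be restarted.
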(fn `Conversation`
  (`self.SetDialogueTreeIndex` "None")
  (`parent.Conversation`))

(fn `Dialogue`
  ;[0.15 0.08514 0.1455 0.5] Create Dialogue and Options that will be added to widget
  (`parent.Dialogue`)
  (switch `name` (`self.ActiveDialogueBranch`)
    (:`Default`
      (bind _state (`self.AddDialogue` "Cafeteria Lady" "Hello" (`|MakeArray` "Hi" :!type "Text")))
      (switch `/Game/Evelyn/Dialogue_Bluprints/Enum_Dialogue` _state
        (:`NewEnumerator0`
          (bind _returnvalue (`GameplayStatics.GetActorOfClass` "/Game/Kyra/BP/BP_Coffee.BP_Coffee_C"))
          (if (`/Game/Kyra/BP/BP_Coffee.Interacted` _returnvalue)
            (bind (_state_2 _optionindex) (`self.AddDialogue` "Cafeteria Lady" "Is there something I can help you with?" (`|MakeArray` "The coffee machine is broken..." :!type "Text")))
            (switch `/Game/Evelyn/Dialogue_Bluprints/Enum_Dialogue` _state_2
              (:`NewEnumerator0`
                (switch `int` _optionindex
                  (:`0`
                    (bind _state_3 (`self.AddDialogue` "Cafeteria Lady" "Oh I see! It's a bit old dear. Just give it a good whack." (`|MakeArray` "I see...thank you." :!type "Text")))
                    (switch `/Game/Evelyn/Dialogue_Bluprints/Enum_Dialogue` _state_3
                      (:`NewEnumerator0`
                        (`self.ClearDialogueProgress`) ; Clears
                        (`self.CloseConversation`) ; Ends the conversation, can be restarted....
                      ))))))
            (else
              (bind _state_4 (`self.AddDialogue` "Cafeteria Lady" "Pardon me...but you don't look so well dear. Maybe you should go get something to drink." (`|MakeArray` "*nods*" :!type "Text")))
              (switch `/Game/Evelyn/Dialogue_Bluprints/Enum_Dialogue` _state_4
                (:`NewEnumerator0`
                  (`self.ClearDialogueProgress`)
                  (`self.CloseConversation`))))))))))

(fn `NewFunction`)