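; Dialogue component for the coffee machine, scripting the player's attempts to get coffee from the broken machine.
; Its Dialogue override chains AddDialogue lines and options, gated on whether NPC_CafeteriaLady has been interacted with.
; If so, whacking revives the machine and grabbing coffee ends the conversation and calls PromptPlayer on BP_Vending; otherwise the player can only leave.
; Conversation resets the dialogue tree index before running the parent logic.
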(fn `Conversation`
  (`self.SetDialogueTreeIndex` "None")
  (`parent.Conversation`))

(fn `Dialogue`
  ;[0.15 0.08514 0.1455 0.5] Create Dialogue and Options that will be added to widget
  (`parent.Dialogue`)
  (switch `name` (`self.ActiveDialogueBranch`)
    (:`Default`
      (bind _state (`self.AddDialogue` "Coffee Machine" "Hmmm it seems to not be working..." (`|MakeArray` "*Pushes buttons*" :!type "Text")))
      (switch `/Game/Evelyn/Dialogue_Bluprints/Enum_Dialogue` _state
        (:`NewEnumerator0`
          (bind _returnvalue (`GameplayStatics.GetActorOfClass` "/Game/Evelyn/Dialogue_Bluprints/NPCs/NPC_CafeteriaLady.NPC_CafeteriaLady_C"))
          (if (`/Game/Evelyn/Dialogue_Bluprints/NPCs/NPC_CafeteriaLady.Interacted` _returnvalue)
            (bind (_state_2 _optionindex) (`self.AddDialogue` "Coffee Machine" "Yup....itsn't working" (`|MakeArray` "*whacks it*" :!type "Text")))
            (switch `/Game/Evelyn/Dialogue_Bluprints/Enum_Dialogue` _state_2
              (:`NewEnumerator0`
                (switch `int` _optionindex
                  (:`0`
                    (bind _state_3 (`self.AddDialogue` "Linda" "+bzzzzz* The coffee machine comes to life" (`|MakeArray` "*Grab coffee*" :!type "Text")))
                    (switch `/Game/Evelyn/Dialogue_Bluprints/Enum_Dialogue` _state_3
                      (:`NewEnumerator0`
                        (`self.ClearDialogueProgress`) ; Clears
                        (`self.CloseConversation`) ; Ends the conversation, can be restarted....
                        (bind _returnvalue_2 (`GameplayStatics.GetActorOfClass` "/Game/Kyra/BP/BP_Vending.BP_Vending_C"))
                        (`/Game/Kyra/BP/BP_Vending.PromptPlayer` _returnvalue_2)))))))
            (else
              (bind _state_4 (`self.AddDialogue` "Coffee Machine" "...." (`|MakeArray` "*Leave*" :!type "Text")))
              (switch `/Game/Evelyn/Dialogue_Bluprints/Enum_Dialogue` _state_4
                (:`NewEnumerator0`
                  (`self.ClearDialogueProgress`)
                  (`self.CloseConversation`))))))))))

(fn `NewFunction`)