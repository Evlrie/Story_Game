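; Dialogue component for the player's purse, where placing a snack in the bag reveals that Lily's ring is missing.
; Dialogue extends the parent and checks BP_Coffee's Interacted flag to choose that two-step exchange or a placeholder purse line.
; AddDialogue pass-through states chain the steps, then progress is cleared and the conversation closes.
; Conversation resets the dialogue tree index to None before calling the parent.
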(fn `Conversation`
  (`self.SetDialogueTreeIndex` "None")
  (`parent.Conversation`))

(fn `Dialogue`
  ;[0.15 0.08514 0.1455 0.5] Create Dialogue and Options that will be added to widget
  (`parent.Dialogue`)
  (switch `name` (`self.ActiveDialogueBranch`)
    (:`Default`
      (bind _returnvalue (`GameplayStatics.GetActorOfClass` "/Game/Kyra/BP/BP_Coffee.BP_Coffee_C"))
      (if (`/Game/Kyra/BP/BP_Coffee.Interacted` _returnvalue)
        (`/Engine/EditorBlueprintResources/StandardMacros.DoOnce` false
          (:`Completed`
            (bind (_state _optionindex) (`self.AddDialogue` "Your Purse" "You open a small pouch of your bag" (`|MakeArray` "Place snack into bag." :!type "Text")))
            (switch `/Game/Evelyn/Dialogue_Bluprints/Enum_Dialogue` _state
              (:`NewEnumerator0`
                (switch `int` _optionindex
                  (:`0`
                    (bind _state_2 (`self.AddDialogue` "Coffee Machine" "Something seems to be missing!" (`|MakeArray` "Where is Lily's ring?!" :!type "Text")))
                    (switch `/Game/Evelyn/Dialogue_Bluprints/Enum_Dialogue` _state_2
                      (:`NewEnumerator0`
                        (`self.ClearDialogueProgress`) ; Clears
                        (`self.CloseConversation`) ; Ends the conversation, can be restarted....
                      ))))))))
        (else
          (bind _state_3 (`self.AddDialogue` "Coffee Machine" "Your purse" (`|MakeArray` "..." :!type "Text")))
          (switch `/Game/Evelyn/Dialogue_Bluprints/Enum_Dialogue` _state_3
            (:`NewEnumerator0`
              (`self.ClearDialogueProgress`)
              (`self.CloseConversation`))))))))

(fn `NewFunction`)