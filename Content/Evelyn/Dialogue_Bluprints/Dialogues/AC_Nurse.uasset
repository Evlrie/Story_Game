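; AC_Nurse is a dialogue component holding the player's conversation with the Nurse about their head injury, the accident and Lily's condition.
; Its Dialogue override calls the parent, then chains AddDialogue nodes, branching on state and chosen option index.
; The opening line offers a leave option, while later lines have single replies.
; Both endings clear dialogue progress and close the conversation, allowing a restart.
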(fn `Dialogue`
  ;[0.15 0.08514 0.1455 0.5] Create Dialogue and Options that will be added to widget
  (`parent.Dialogue`)
  (switch `name` (`self.ActiveDialogueBranch`)
    (:`Default`
      (bind (_state _optionindex) (`self.AddDialogue` "Nurse" "How's your head?" (`|MakeArray` "Hurts, but other than that I'm fine..." "*Leave*" :!type "Text")))
      (switch `/Game/Evelyn/Dialogue_Bluprints/Enum_Dialogue` _state
        (:`NewEnumerator0`
          (switch `int` _optionindex
            (:`0`
              (bind (_state_2 _optionindex_2) (`self.AddDialogue` "Nurse" "Let the doc know if you notice any changes." (`|MakeArray` "I will." :!type "Text")))
              (switch `/Game/Evelyn/Dialogue_Bluprints/Enum_Dialogue` _state_2
                (:`NewEnumerator0`
                  (switch `int` _optionindex_2
                    (:`0`
                      (bind (_state_3 _optionindex_3) (`self.AddDialogue` "Nurse" "It's a damn miracle you're up and about after an accident like that..." (`|MakeArray` "How is Lily?" :!type "Text")))
                      (switch `/Game/Evelyn/Dialogue_Bluprints/Enum_Dialogue` _state_3
                        (:`NewEnumerator0`
                          (switch `int` _optionindex_3
                            (:`0`
                              (bind _state_4 (`self.AddDialogue` "Nurse" "It's hard to say just yet... but we're doing all we can for her." (`|MakeArray` "Thank you...." :!type "Text")))
                              (switch `/Game/Evelyn/Dialogue_Bluprints/Enum_Dialogue` _state_4
                                (:`NewEnumerator0`
                                  (`self.ClearDialogueProgress`) ; Clears
                                  (`self.CloseConversation`) ; Ends the conversation, can be restarted....
                                )))))))))))
            (:`1`
              (`self.ClearDialogueProgress`) ; Clears
              (`self.CloseConversation`) ; Ends the conversation, can be restarted....
            )))))))