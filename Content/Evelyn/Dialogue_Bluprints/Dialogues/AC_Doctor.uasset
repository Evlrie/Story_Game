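; Dialogue component for the Doctor, who turns the player away during an emergency and deflects questions about Lilly.
; Overrides Dialogue, calling the parent and switching on the active branch, then nesting AddDialogue calls whose chosen option index selects the next line.
; Both the immediate leave option and the final escort line clear dialogue progress and close the conversation, while BeginPlay and Tick are unused.
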(fn `Dialogue`
  ;[0.15 0.08514 0.1455 0.5] Create Dialogue and Options that will be added to widget
  (`parent.Dialogue`)
  (switch `name` (`self.ActiveDialogueBranch`)
    (:`Default`
      (bind (_state _optionindex) (`self.AddDialogue` "Doctor" "Ma'am you can't be out here there is an emergency." (`|MakeArray` "What is happening?!" "*Leave*" :!type "Text")))
      (switch `/Game/Evelyn/Dialogue_Bluprints/Enum_Dialogue` _state
        (:`NewEnumerator0`
          (switch `int` _optionindex
            (:`0`
              (bind (_state_2 _optionindex_2) (`self.AddDialogue` "Doctor" "I can't tell you" (`|MakeArray` "Is it Lilly?!" :!type "Text")))
              (switch `/Game/Evelyn/Dialogue_Bluprints/Enum_Dialogue` _state_2
                (:`NewEnumerator0`
                  (switch `int` _optionindex_2
                    (:`0`
                      (bind _state_3 (`self.AddDialogue` "Doctor" "Could someone please escort this lady to to consultation room?!" (`|MakeArray` "leave" :!type "Text")))
                      (switch `/Game/Evelyn/Dialogue_Bluprints/Enum_Dialogue` _state_3
                        (:`NewEnumerator0`
                          (`self.ClearDialogueProgress`) ; Clears
                          (`self.CloseConversation`) ; Ends the conversation, can be restarted....
                        )))))))
            (:`1`
              (`self.ClearDialogueProgress`) ; Clears
              (`self.CloseConversation`) ; Ends the conversation, can be restarted....
            )))))))