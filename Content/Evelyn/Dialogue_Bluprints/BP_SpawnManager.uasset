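; BP_SpawnManager is a manager actor that spawns a BP_LillyRing at every BP_Spawner in the level.
; On BeginPlay it gathers all BP_Spawner actors into a Spawners array, then calls its SpawnRing event.
; SpawnRing loops over that array and spawns a ring at each spawner root's world location and rotation, with debug prints marking both steps.
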(event `self.ReceiveBeginPlay`
  (`KismetSystemLibrary.PrintString` "manager activated")
  (bind _outactors (`GameplayStatics.GetAllActorsOfClass` "/Game/Evelyn/Dialogue_Bluprints/BP_Spawner.BP_Spawner_C"))
  (set `self.spawners` _outactors)
  (`self.Spawn Ring`))

(event `Spawn Ring`
  (`KismetSystemLibrary.PrintString` "ayo it works")
  (for _array_element (`self.spawners`)
    (bind (_returnvalue_location _returnvalue_rotation) (`KismetMathLibrary.BreakTransform` (`SceneComponent.K2_GetComponentToWorld` (`/Game/Evelyn/Dialogue_Bluprints/BP_Spawner.DefaultSceneRoot` _array_element))))
    (`|SpawnActorFromClass` "/Game/Evelyn/BP_LillyRing.BP_LillyRing_C" (`KismetMathLibrary.MakeTransform` _returnvalue_location _returnvalue_rotation) "Undefined" "MultiplyWithRoot" null null)))

(fn `UserConstructionScript`)