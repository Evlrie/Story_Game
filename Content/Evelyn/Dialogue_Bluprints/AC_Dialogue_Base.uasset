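; Base dialogue component that runs branching conversations through a W_Dialogue widget and notifies its owner on close.
; The Dialogue function holds only a blank AddDialogue call, apparently meant for child overrides.
; Each selection is stored in DialogueProgress, then Dialogue replays from the start: AddDialogue returns saved choices for answered steps and updates the widget otherwise.
; Helpers rewind or clear progress, and changing the tree index clears it.
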(fn `AddDialogue`
  (params (Speaker :type Text) (Dialogue :type Text) (`Options Text` :type "Array of Text"))
  (returns (State :type "/Game/Evelyn/Dialogue_Bluprints/Enum_Dialogue Enum") (OptionIndex :type Integer))
  (bind (_value _returnvalue) (`BlueprintMapLibrary.Map_Find` (`self.DialogueProgress`) (`self.DialogueIndex`)))
  (`/Engine/EditorBlueprintResources/StandardMacros.IncrementInt` (`self.DialogueIndex`) ; Increments Dialogue by 1
    (:`  `
      (if _returnvalue
        (return "NewEnumerator0" _value)
        (else
          (`/Game/UI/W_Dialogue.Update Dialogue` (`self.DialogueWidget`) (`self.DialogueIndex`) (`local.Speaker`) (`local.Dialogue`) (`local.Options Text`))
          (return "NewEnumerator1" 0) ; Updates Dialogue
        )))))

(fn `ClearDialogueProgress`
  (`BlueprintMapLibrary.Map_Clear` (`self.DialogueProgress`)))

(fn `CloseConversation`
  ;[0.15 0.07109 0.07109 0.5] Closes Conversation
  (`Widget.RemoveFromParent` (`self.DialogueWidget`)) ; Will remove the dialogue from the widget when closed
  (message `/Game/Evelyn/Dialogue_Bluprints/BP_Interaction.Conversation Closed` (`self.GetOwner`)))

(fn `Conversation`
  (bind _returnvalue (`|CreateWidget` "/Game/UI/W_Dialogue.W_Dialogue_C" null self))
  (bind _output_get (set `self.DialogueWidget` _returnvalue))
  (`UserWidget.AddToViewport` _output_get 0)
  (`self.Progress Dialogue`))

(fn `Dialogue`
  (`self.AddDialogue` ""))

(fn `Progress Dialogue`
  (set `self.DialogueIndex` -1)
  (`self.Dialogue`))

(fn `RemoveDialogueProgress`
  (params (`Progress Steps` :type Integer))
  (for _index (range (+ `Progress Steps` 1))
    (`BlueprintMapLibrary.Map_Remove` (`self.DialogueProgress`) (- (`self.DialogueIndex`) _index))))

(fn `SetDialogueTreeIndex`
  (params (DialogueTreeIndex :type Integer))
  ;[0.05624 0.15 0.04141 0.5] Controls Dialogue Branches in Convo
  (set `self.DialogueTreeIndex` DialogueTreeIndex)
  (`self.ClearDialogueProgress`))

(fn `UpdateSelectedOption`
  (params (`Progress Index` :type "Integer (by ref)") (`Options Index` :type "Integer (by ref)"))
  (`BlueprintMapLibrary.Map_Add` (`self.DialogueProgress`) `Progress Index` `Options Index`)
  (`self.Progress Dialogue`))