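; BP_DizzySpells is a one-shot trigger that gives the player a dizzy spell with accompanying thought text.
; Beginning overlap enables post-process volumes tagged DizzyPP, and ending overlap disables them, each gated by its own DoOnce.
; For each volume found, both events also create a thought widget remarking on the onset or recovery, with a short Delay before removing it.
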(event `self.Trigger.OnComponentBeginOverlap`
  (params (OverlappedComponent :type "PrimitiveComponent Object Reference") (OtherActor :type "Actor Object Reference") (OtherComp :type "PrimitiveComponent Object Reference") (OtherBodyIndex :type Integer) (bFromSweep :type Boolean) (SweepResult :type "HitResult Structure (by ref)"))
  (`/Engine/EditorBlueprintResources/StandardMacros.DoOnce` false
    (:`Completed`
      (bind _outactors (`GameplayStatics.GetAllActorsOfClassWithTag` "/Script/Engine.PostProcessVolume" "DizzyPP"))
      (for _array_element _outactors
        (set `PostProcessVolume.bEnabled` true _array_element)
        (bind _returnvalue (`|CreateWidget` "/Game/UI/W_Thoughts.W_Thoughts_C"))
        (`/Game/UI/W_Thoughts.Think` _returnvalue "My head....")
        (`UserWidget.AddToViewport` _returnvalue 0)
        (`KismetSystemLibrary.Delay` 3.0)
        (`Widget.RemoveFromParent` _returnvalue)))))

(event `self.Trigger.OnComponentEndOverlap`
  (params (OverlappedComponent :type "PrimitiveComponent Object Reference") (OtherActor :type "Actor Object Reference") (OtherComp :type "PrimitiveComponent Object Reference") (OtherBodyIndex :type Integer))
  (`/Engine/EditorBlueprintResources/StandardMacros.DoOnce` false
    (:`Completed`
      (bind _outactors (`GameplayStatics.GetAllActorsOfClassWithTag` "/Script/Engine.PostProcessVolume" "DizzyPP"))
      (for _array_element _outactors
        (set `PostProcessVolume.bEnabled` false _array_element)
        (bind _returnvalue (`|CreateWidget` "/Game/UI/W_Thoughts.W_Thoughts_C"))
        (`/Game/UI/W_Thoughts.Think` _returnvalue "I feel better now...must be from stress.")
        (`UserWidget.AddToViewport` _returnvalue 0)
        (`KismetSystemLibrary.Delay` 3.0)
        (`Widget.RemoveFromParent` _returnvalue)))))

(fn `UserConstructionScript`)